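; Player character Blueprint for AshForest that adds the UI layer on top of its parent class's lock-on, checkpoint and respawn logic.
; BeginPlay creates and initializes the PlayerHUD, which refreshes dash charges every Tick and is notified of checkpoint updates and respawns.
; A lock-on widget is created on demand, spins on target change, follows the target's projected screen position each frame, and hides when projection fails.
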(event EventOnLockonTargetUpdated
  (|CallParentFunction)
  (Utilities|IsValid (Variables|Default|GetLockOnTarget_Current)
    (:Is%20Valid
      (CallFunction|UpdateLockonWidget)
      (bind _aslock_on_widget (Utilities|Casting|CastToLockOnWidget (Variables|Default|GetCurrLockOnWidget)))
      (Default|PlaySpinAnim _aslock_on_widget))
    (:Is%20Not%20Valid
      (Utilities|IsValid (Variables|Default|GetCurrLockOnWidget)
        (:Is%20Valid
          (Widget|RemovefromParent (Variables|Default|GetCurrLockOnWidget))
          (Variables|Default|SetCurrLockOnWidget 0))))))

(event EventOnCheckpointUpdated
  (|CallParentFunction)
  (bind _asplayer_hud (Utilities|Casting|CastToPlayerHUD (Variables|Default|GetCurrHUDWidget)))
  (Default|OnCheckpointUpdated _asplayer_hud))

(event EventBeginPlay
  (|CallParentFunction)
  (if (== (Variables|Default|GetCurrHUDWidget) 0)
    (bind _asplayer_controller (Utilities|Casting|CastToPlayerController (Pawn|GetController)))
    (bind _returnvalue (UserInterface|CreateWidget "/Game/_AshForest/HUD/PlayerHUD.PlayerHUD_C" _asplayer_controller))
    (UserInterface|Viewport|AddtoViewport _returnvalue 0)
    (Default|InitHUD _returnvalue self)
    (Variables|Default|SetCurrHUDWidget _returnvalue)))

(event EventTick
  (params (DeltaSeconds :type Float%20%28single-precision%29))
  (|CallParentFunction DeltaSeconds)
  (CallFunction|UpdateLockonWidget)
  (bind _asplayer_hud (Utilities|Casting|CastToPlayerHUD (Variables|Default|GetCurrHUDWidget)))
  (Default|UpdateDashCharges _asplayer_hud))

(event EventOnRespawned
  (|CallParentFunction)
  (bind _asplayer_hud (Utilities|Casting|CastToPlayerHUD (Variables|Default|GetCurrHUDWidget)))
  (Default|OnRespawn _asplayer_hud))

(fn ConstructionScript)

(fn UpdateLockonWidget
  (bind _lockontarget_current (Variables|Default|GetLockOnTarget_Current))
  (bind _asplayer_controller (Utilities|Casting|CastToPlayerController (Pawn|GetController)))
  (if (!= _lockontarget_current 0)
    (Utilities|IsValid (Variables|Default|GetCurrLockOnWidget)
      (:Is%20Valid
        _)
      (:Is%20Not%20Valid
        (bind _returnvalue (UserInterface|CreateWidget "/Game/_AshForest/HUD/LockOnWidget.LockOnWidget_C" _asplayer_controller))
        (bind _output_get (Variables|Default|SetCurrLockOnWidget _returnvalue))
        (UserInterface|Viewport|AddtoViewport _output_get 0)))
    (if (.ReturnValue (Class|WidgetLayoutLibrary|ProjectWorldLocationtoWidgetPosition _asplayer_controller (Transformation|GetWorldLocation _lockontarget_current)))
      (Widget|SetVisibility (Variables|Default|GetCurrLockOnWidget) "HitTestInvisible")
      (Class|Widget|SetRenderTranslation (Variables|Default|GetCurrLockOnWidget) (.ScreenPosition (Class|WidgetLayoutLibrary|ProjectWorldLocationtoWidgetPosition _asplayer_controller (Transformation|GetWorldLocation _lockontarget_current))))
      (else
        (Widget|SetVisibility (Variables|Default|GetCurrLockOnWidget) "Hidden")))))