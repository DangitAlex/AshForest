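; Unstable platform that wiggles when an AshForest character lands on it, then collapses and later resets.
; A collision box hit on the top face plays a rate-scaled timeline that bobs the mesh vertically for the collapse delay.
; It then disables collision, and Tick drops the mesh until the fall duration ends, snapping it back and restoring collision.
; The construction script fits the box to the mesh's bounds and scale.
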(event OnComponentHit(PlatformCollision)
  (params (HitComponent :type Primitive%20Component%20Object%20Reference) (OtherActor :type Actor%20Object%20Reference) (OtherComp :type Primitive%20Component%20Object%20Reference) (NormalImpulse :type Vector :default "0, 0, 0") (Hit :type Hit%20Result%20Structure%20%28by%20ref%29))
  (bind _collapsetimeline (Variables|Default|GetCollapseTimeline))
  (bind _staticmesh (Variables|Default|GetStaticMesh))
  (bind _timeuntilcollapse (Variables|Default|GetTimeUntilCollapse))
  (bind _relativelocation (Variables|/Script/Engine.SceneComponent|GetRelativeLocation _staticmesh))
  (if (and (not (Audio|Components|Audio|IsPlaying _collapsetimeline)) (Variables|Default|GetbHasReset))
    (if (Utilities|ClassIsChildOf (Utilities|GetClass OtherActor) "/Script/AshForest.AshForestCharacter")
      (if (> (Math|Vector|DotProduct (Math|Vector|NegateVector (.ImpactNormal (Collision|BreakHitResult Hit))) (Transformation|GetActorUpVector)) 0.75)
        (Components|Timeline|SetPlayRate _collapsetimeline (* (/ (Components|Timeline|GetTimelineLength _collapsetimeline) _timeuntilcollapse) (Variables|Default|GetWigglePlayRate)))
        (Utilities|FlowControl|Sequence
          (:then_0
            (bind _floorz (Timeline|CollapseTimeline PlayFromStart)
              (:Update
                (Transformation|SetRelativeLocation _staticmesh (Math|Vector|MakeVector (.x _relativelocation) (.y _relativelocation) (* _floorz (Variables|Default|GetWiggleDist))) false false))))
          (:then_1
            (Utilities|FlowControl|Delay _timeuntilcollapse)
            (Audio|Components|Audio|Stop _collapsetimeline)
            (Variables|Default|SetLastFallStartTime (Utilities|Time|GetGameTimeinSeconds))
            (Collision|SetCollisionEnabled (Variables|Default|GetPlatformCollision) "NoCollision")
            (Variables|Default|SetbHasReset false)))))))

(event EventTick
  (params (DeltaSeconds :type Float%20%28single-precision%29))
  (bind _staticmesh (Variables|Default|GetStaticMesh))
  (|CallParentFunction DeltaSeconds)
  (if (not (Variables|Default|GetbHasReset))
    (Transformation|AddRelativeLocation _staticmesh (Math|Vector|MakeVector 0.0 0.0 (* DeltaSeconds (Variables|Default|GetFallSpeed) -1.0)) false false)
    (if (>= (- (Utilities|Time|GetGameTimeinSeconds) (Variables|Default|GetLastFallStartTime)) (Variables|Default|GetFallDuration))
      (Variables|Default|SetbHasReset true)
      (Transformation|SetRelativeLocation _staticmesh "0, 0, 0" false false)
      (Collision|SetCollisionEnabled (Variables|Default|GetPlatformCollision) "QueryAndPhysics"))))

(fn ConstructionScript
  (bind _platformcollision (Variables|Default|GetPlatformCollision))
  (bind _staticmesh (Variables|Default|GetStaticMesh))
  (|CallParentFunction)
  (Components|Box|SetBoxExtent _platformcollision (.boxextent (StaticMesh|GetBounds (Variables|/Script/Engine.StaticMeshComponent|GetStaticMesh _staticmesh))) true)
  (Transformation|SetWorldScale3D _platformcollision (Transformation|GetWorldScale _staticmesh)))