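; Checkpoint Blueprint for Ash Forest whose construction script provides placement aids and index assignment.
; It draws a temporary green debug line to its assigned RespawnPoint, flushing older persistent lines first.
; When UpdateCheckpointIndex is set or the index is negative, it scans all other AshForestCheckpoint actors and takes one above the highest index.
; UpdateCheckpointIndex resets itself, acting as an editor-style button for renumbering.
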(fn ConstructionScript
  (bind _respawnpoint (Variables|Default|GetRespawnPoint))
  (|CallParentFunction)
  (Utilities|FlowControl|Sequence
    (:then_0
      (if (!= _respawnpoint 0)
        (Rendering|Debug|FlushPersistentDebugLines)
        (Rendering|Debug|DrawDebugLine (Transformation|GetActorLocation) (Transformation|GetActorLocation _respawnpoint) "(R=0.091340,G=1.000000,B=0.000000,A=1.000000)" 1e+01 1e+01)))
    (:then_1
      (if (or (Variables|Checkpoint|GetbUpdateCheckpointIndex) (< (Class|AshForestCheckpoint|GetCheckpointIndex) 0))
        (Variables|Checkpoint|SetbUpdateCheckpointIndex false)
        (LocalVariables|SethighestIndex -1)
        (bind _outactors (Actor|GetAllActorsOfClass "/Script/AshForest.AshForestCheckpoint"))
        (for _array_element _outactors
          (if (!= _array_element self)
            (if (> (Class|AshForestCheckpoint|GetCheckpointIndex _array_element) (LocalVariables|GethighestIndex))
              (LocalVariables|SethighestIndex (Class|AshForestCheckpoint|GetCheckpointIndex _array_element)))))
        (Variables|Default|SetCheckpointIndex (+ (LocalVariables|GethighestIndex) 1))))))