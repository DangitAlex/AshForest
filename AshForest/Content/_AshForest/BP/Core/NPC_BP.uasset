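; NPC that acts as a toll gate, unlocking linked objects when the AshForestCharacter overlaps it while carrying big-unit money.
; While locked, an overlap reveals its text, spends one big unit if available, sends Activate to each OpensDoors entry, shows the eyeball and disables collision.
; A sequence then switches text and color to the locked or unlocked state.
; The construction script drops the mesh to the collision bottom and applies default text.
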(event Collision|EventActorBeginOverlap
  (params (OtherActor :type Actor%20Object%20Reference))
  (if (Variables|Default|GetbLocked)
    (bind _asash_forest_character (Utilities|Casting|CastToAshForestCharacter OtherActor))
    (Development|SetHiddeninGame (Variables|Default|GetTextRender) false false)
    (Utilities|FlowControl|Sequence
      (:then_0
        (if (> (Variables|/Script/AshForest.AshForestCharacter|GetCurrentBigUnitMoniez _asash_forest_character) 0)
          (Math|Integer|DecrementInt (Variables|/Script/AshForest.AshForestCharacter|GetCurrentBigUnitMoniez _asash_forest_character)
            (:%20%20
              (Variables|Default|SetbLocked false)
              (for _array_element (Variables|Default|GetOpensDoors)
                (Class|ActivateableInterface|Activate(Message) _array_element self))
              (Development|SetHiddeninGame (Variables|Default|GetEyeball) false false)
              (Collision|SetCollisionEnabled (Variables|Default|GetCollisionComponent) "NoCollision")))))
      (:then_1
        (CallFunction|NPCUpdateText)))))

(event EventBeginPlay
  (|CallParentFunction)
  (CallFunction|NPCSetTexttoDefault)
  (Variables|Default|SetbLocked true))

(fn ConstructionScript
  (bind _skeletalmesh (Variables|Default|GetSkeletalMesh))
  (bind _relativelocation (Variables|/Script/Engine.SceneComponent|GetRelativeLocation _skeletalmesh))
  (|CallParentFunction)
  (Transformation|SetRelativeLocation _skeletalmesh (Math|Vector|MakeVector (.x _relativelocation) (.y _relativelocation) (* (.z (.BoxExtent (Collision|GetComponentBounds (Variables|Default|GetCollisionComponent)))) -1.0)) false false)
  (CallFunction|NPCSetTexttoDefault))

(fn NPCUpdateText
  (bind _textrender (Variables|Default|GetTextRender))
  (if (Variables|Default|GetbLocked)
    (Rendering|Components|TextRender|SetText _textrender (Variables|Default|GetNPC%20Text_Locked))
    (Rendering|Components|TextRender|SetTextRenderColor _textrender (Math|Conversions|ToColor(LinearColor) (Variables|Default|GetTextColor_Locked)))
    (else
      (Rendering|Components|TextRender|SetText _textrender (Variables|Default|GetNPC%20Text_Unlocked))
      (Rendering|Components|TextRender|SetTextRenderColor _textrender (Math|Conversions|ToColor(LinearColor) (Variables|Default|GetTextColor_Unlocked))))))

(fn NPCSetTexttoDefault
  (bind _textrender (Variables|Default|GetTextRender))
  (Rendering|Components|TextRender|SetText _textrender (Variables|Default|GetNPC%20Text_Default))
  (Rendering|Components|TextRender|SetTextRenderColor _textrender (Math|Conversions|ToColor(LinearColor) "(R=1.000000,G=0.869393,B=0.000000,A=1.000000)")))