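; AshForestCreatureBP is a creature Blueprint that adds particle feedback for damage and death on top of its parent class behavior.
; On damage it calls the parent handler, then, if health remains above zero, spawns a spark burst at the impact point oriented along the hit normal.
; On targetable death it calls the parent handler and spawns an explosion at the actor's location.
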(event EventTakeDamage
  (params (DamageCauser :type Actor%20Object%20Reference) (DamageAmount :type Float%20%28single-precision%29%20%28by%20ref%29) (DamageHitEvent :type Hit%20Result%20Structure%20%28by%20ref%29))
  (bind (_bblockinghit _binitialoverlap _time _distance _location _impactpoint _normal _impactnormal) (Collision|BreakHitResult DamageHitEvent))
  (|CallParentFunction DamageCauser DamageAmount DamageHitEvent)
  (if (> (Variables|Default|GetCurrentHealth) 0.0)
    (Effects|SpawnEmitteratLocation "/Game/StarterContent/Particles/P_SparkBurst.P_SparkBurst" _impactpoint (Math|Conversions|RotationFromXVector _impactnormal) (Math|Conversions|ToVector(Float) 1.5))))

(event EventOnTargetableDeath
  (params (Murderer :type Actor%20Object%20Reference))
  (|CallParentFunction Murderer)
  (Effects|SpawnEmitteratLocation "/Game/StarterContent/Particles/P_Explosion.P_Explosion" (Transformation|GetActorLocation)))

(fn ConstructionScript)