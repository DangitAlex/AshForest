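; Collectable money pickup that adds to the Ash Forest character's currency on overlap, then spawns a collected effect and destroys itself.
; A flag picks the big or small counter, and big pickups also unhide the character's eye mesh.
; A timeline holds the mesh's yaw spin and height bob logic, with scalable speed and height, though no Play call is wired to it.
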(event Collision|EventActorBeginOverlap
  (params (OtherActor :type Actor%20Object%20Reference))
  (bind _asash_forest_character_bp (Utilities|Casting|CastToAshForestCharacterBP OtherActor))
  (if (Variables|Default|GetbIsBigCollectible)
    (Math|Integer|IncrementInt (Variables|/Script/AshForest.AshForestCharacter|GetCurrentBigUnitMoniez _asash_forest_character_bp)
      (:%20%20
        (Development|SetHiddeninGame (Variables|/Game/_AshForest/BP/Core/AshForestCharacterBP.AshForestCharacterBP_C|GetEyeMesh _asash_forest_character_bp) false false)))
    (else
      (Math|Integer|IncrementInt (Variables|/Script/AshForest.AshForestCharacter|GetCurrentSmolMoniez _asash_forest_character_bp)
        (:%20%20
          _))))
  (Effects|SpawnEmitteratLocation (Variables|Default|GetCollectedVFX) (Transformation|GetActorLocation))
  (Actor|DestroyActor))

(event EventBeginPlay
  (|CallParentFunction)
  (Components|Timeline|SetPlayRate (Variables|Default|GetMoneyMoveTimeline) (Variables|Default|GetMoneyMoveSpeedScale)))

(fn ConstructionScript
  (|CallParentFunction))