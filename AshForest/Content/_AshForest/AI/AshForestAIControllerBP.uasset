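; AI controller Blueprint for Ash Forest creatures that starts their behavior tree and records a home location.
; On BeginPlay it initializes AI with the BB_AshForestCreature blackboard and, if that succeeds, runs MainBT.
; It then polls with a short delay until the controlled pawn is valid and writes that pawn's location to the HomeLocation blackboard key.
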(event Custom|Init_AI
  (bind _returnvalue (Pawn|GetControlledPawn))
  (bind (_blackboardcomponent _returnvalue_2) (Class|AIController|UseBlackboard "/Game/_AshForest/AI/BB_AshForestCreature.BB_AshForestCreature"))
  (if _returnvalue_2
    (AI|RunBehaviorTree (Variables|Default|GetMainBT))
    (Utilities|IsValid _returnvalue :!label _label
      (:Is%20Valid
        (AI|Components|Blackboard|SetValueasVector _blackboardcomponent (Utilities|Name|MakeLiteralName "HomeLocation") (Transformation|GetActorLocation _returnvalue)))
      (:Is%20Not%20Valid
        (Utilities|FlowControl|Delay 0.01)
        (goto _label)))))

(event EventBeginPlay
  (CallFunction|InitAI))

(fn ConstructionScript)